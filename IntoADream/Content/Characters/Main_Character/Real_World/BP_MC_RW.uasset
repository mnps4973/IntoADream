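; BP_MC_RW is the player-controlled main character for the Real World, handling basic movement, jumping and camera look.
; On BeginPlay it adds the IMC_Default mapping context to the player controller's Enhanced Input subsystem.
; Input actions drive jump start and stop, movement along the actor's forward and right vectors, and controller yaw and pitch for looking around.
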(event `self.ReceiveBeginPlay`
  ;[1 1 1] Add input controllers
  (bind _asplayer_controller (cast `PlayerController` (`self.GetController`)))
  (bind _returnvalue (pcsubsystem `EnhancedInputLocalPlayerSubsystem` _asplayer_controller))
  (`/Engine/EditorBlueprintResources/StandardMacros.IsValid` _returnvalue
    (:`Is Valid`
      (`EnhancedInputSubsystemInterface.AddMappingContext` _returnvalue "/Game/ThirdPerson/Input/IMC_Default.IMC_Default" 0 (struct)))))

(event `EnhancedInput|/Game/ThirdPerson/Input/Actions/Main_Character_Actions/Jump_Main_Character_IA`
  (params (ActionValue :type Boolean) (ElapsedSeconds :type "Float (double-precision)") (TriggeredSeconds :type "Float (double-precision)") (InputAction :type "InputAction Object Reference" :default "/Game/ThirdPerson/Input/Actions/Main_Character_Actions/Jump_Main_Character_IA.Jump_Main_Character_IA"))
  ;[1 1 1] Handle jump
  (:`Triggered`
    (`self.Jump`))
  (:`Completed`
    (`self.StopJumping`)))

(event `EnhancedInput|/Game/ThirdPerson/Input/Actions/Main_Character_Actions/Move_Main_Character_IA`
  (params (ActionValue :type "Vector2D Structure") (ElapsedSeconds :type "Float (double-precision)") (TriggeredSeconds :type "Float (double-precision)") (InputAction :type "InputAction Object Reference" :default "/Game/ThirdPerson/Input/Actions/Main_Character_Actions/Move_Main_Character_IA.Move_Main_Character_IA"))
  ;[1 1 1] Movement
  (:`Triggered`
    (`self.AddMovementInput` (`self.GetActorRightVector`) ActionValue_X)
    (`self.AddMovementInput` (`self.GetActorForwardVector`) ActionValue_Y)))

(event `EnhancedInput|/Game/ThirdPerson/Input/Actions/Main_Character_Actions/Look_Around_IA`
  (params (ActionValue :type "Vector2D Structure") (ElapsedSeconds :type "Float (double-precision)") (TriggeredSeconds :type "Float (double-precision)") (InputAction :type "InputAction Object Reference" :default "/Game/ThirdPerson/Input/Actions/Main_Character_Actions/Look_Around_IA.Look_Around_IA"))
  ;[1 1 1] Look around
  (:`Triggered`
    (`self.AddControllerYawInput` ActionValue_X)
    (`self.AddControllerPitchInput` ActionValue_Y)))

(fn `UserConstructionScript`)